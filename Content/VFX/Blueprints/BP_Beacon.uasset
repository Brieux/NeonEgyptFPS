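; BP_Beacon is an animated VFX beacon that endlessly cycles through lighting up, opening, closing and powering down from BeginPlay.
; Activation and Desactivation step the Brightness parameter on three pairs of top and bottom neons in staggered sequence.
; Open plays a sound, starts the NSBeaconCeinture effect and uses a timeline to lerp the plates apart vertically.
; Close reverses the movement, stops the effect, then triggers Desactivation, which restarts Activation after a delay.
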(event `self.ReceiveBeginPlay`
  (`self.SetPositionStart`)
  (`self.Activation`))

(event `SetPositionStart`
  (bind (_returnvalue_x _returnvalue_y _returnvalue_z) (`KismetMathLibrary.BreakVector` (`SceneComponent.K2_GetComponentLocation` (`self.SM_Beacon_01_PlateTop`))))
  (bind (_returnvalue_x_2 _returnvalue_y_2 _returnvalue_z_2) (`KismetMathLibrary.BreakVector` (`SceneComponent.K2_GetComponentLocation` (`self.SM_Beacon_01_PlateBot`))))
  ;[0.8385 0.4826 0 1 32] SET POSITION
  (set `self.PositionStartTop` (`SceneComponent.K2_GetComponentLocation` (`self.SM_Beacon_01_PlateTop`)))
  (set `self.PositionStartBot` (`SceneComponent.K2_GetComponentLocation` (`self.SM_Beacon_01_PlateBot`)))
  (set `self.PositionEndTop` (`KismetMathLibrary.MakeVector` _returnvalue_x _returnvalue_y (+ _returnvalue_z 60.0)))
  (set `self.PositionEndBot` (`KismetMathLibrary.MakeVector` _returnvalue_x_2 _returnvalue_y_2 (- _returnvalue_z_2 60.0))))

(event `self.ReceiveTick`
  (params (DeltaSeconds :type "Float (single-precision)")))

(event `Open`
  ;[0.1503 1 0 1 32] OPEN ANIMATION
  (`GameplayStatics.PlaySoundAtLocation` "/Game/Audio/AMB/SC_Neon_01.SC_Neon_01" (`SceneComponent.K2_GetComponentLocation` (`self.SM_Beacon_01_Center`)) (struct) 1.0 1.0 0.0 null null null null)
  (if (not (`self.Open?`))
    (set `self.Open?` true)
    (`ActorComponent.Activate` (`self.NS_Beacon_Ceinture`) true)
    (bind (_direction _displacementverticale) (`Timeline|Timeline_Opening` :!via `PlayFromStart`)
      (:`Update`
        (`SceneComponent.K2_SetWorldLocation` (`self.SM_Beacon_01_PlateBot`) (`KismetMathLibrary.VLerp` (`self.PositionStartBot`) (`self.PositionEndBot`) _displacementverticale) false false)
        (`SceneComponent.K2_SetWorldLocation` (`self.SM_Beacon_01_PlateTop`) (`KismetMathLibrary.VLerp` (`self.PositionStartTop`) (`self.PositionEndTop`) _displacementverticale) false false))
      (:`Finished`
        (`KismetSystemLibrary.Delay` 1.0)
        (`self.Close`)))))

(event `Close`
  ;[1 0.04167 0.04167 1 32] Comment
  (if (`self.Open?`)
    (set `self.Open?` false)
    (bind (_direction _displacementverticale) (`Timeline|Timeline_Closing` :!via `PlayFromStart`)
      (:`Update`
        (`SceneComponent.K2_SetWorldLocation` (`self.SM_Beacon_01_PlateBot`) (`KismetMathLibrary.VLerp` (`self.PositionEndBot`) (`self.PositionStartBot`) _displacementverticale) false false)
        (`SceneComponent.K2_SetWorldLocation` (`self.SM_Beacon_01_PlateTop`) (`KismetMathLibrary.VLerp` (`self.PositionEndTop`) (`self.PositionStartTop`) _displacementverticale) false false))
      (:`Finished`
        (`ActorComponent.Deactivate` (`self.NS_Beacon_Ceinture`))
        (`KismetSystemLibrary.Delay` 1.0)
        (`self.Desactivation`)))))

(event `Activation`
  ;[0.1503 1 0 1 32] OPEN ANIMATION
  (`MeshComponent.SetScalarParameterValueOnMaterials` (`self.SM_Beacon_01_NeonTop3`) "Brightness" 3.0)
  (`MeshComponent.SetScalarParameterValueOnMaterials` (`self.SM_Beacon_01_NeonBot3`) "Brightness" 3.0)
  (`KismetSystemLibrary.Delay` 0.2)
  (`MeshComponent.SetScalarParameterValueOnMaterials` (`self.SM_Beacon_01_NeonTop2`) "Brightness" 3.0)
  (`MeshComponent.SetScalarParameterValueOnMaterials` (`self.SM_Beacon_01_NeonBot2`) "Brightness" 3.0)
  (`KismetSystemLibrary.Delay` 0.2)
  (`MeshComponent.SetScalarParameterValueOnMaterials` (`self.SM_Beacon_01_NeonTop1`) "Brightness" 3.0)
  (`MeshComponent.SetScalarParameterValueOnMaterials` (`self.SM_Beacon_01_NeonBot1`) "Brightness" 3.0)
  (`KismetSystemLibrary.Delay` 0.2)
  (`self.Open`))

(event `Desactivation`
  ;[1 0.04167 0.04167 1 32] Comment
  (`MeshComponent.SetScalarParameterValueOnMaterials` (`self.SM_Beacon_01_NeonBot1`) "Brightness" 0.0)
  (`MeshComponent.SetScalarParameterValueOnMaterials` (`self.SM_Beacon_01_NeonTop1`) "Brightness" 0.0)
  (`KismetSystemLibrary.Delay` 0.2)
  (`MeshComponent.SetScalarParameterValueOnMaterials` (`self.SM_Beacon_01_NeonTop2`) "Brightness" 0.0)
  (`MeshComponent.SetScalarParameterValueOnMaterials` (`self.SM_Beacon_01_NeonBot2`) "Brightness" 0.0)
  (`KismetSystemLibrary.Delay` 0.2)
  (`MeshComponent.SetScalarParameterValueOnMaterials` (`self.SM_Beacon_01_NeonTop3`) "Brightness" 0.0)
  (`MeshComponent.SetScalarParameterValueOnMaterials` (`self.SM_Beacon_01_NeonBot3`) "Brightness" 0.0)
  (`KismetSystemLibrary.Delay` 2.0)
  (`self.Activation`))

(fn `UserConstructionScript`)