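; Capturable beacon actor that charges while the first-person character stands in its sphere and reverses slowly when they leave.
; A timeline turns three neon tiers from red to cyan by threshold on dynamic material instances, while a second fades the zone material in and out.
; At full charge it calls CheckVictory on the player, then plays opening animation and Niagara effect, dims the neons, flies away and destroys itself.
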(event `self.ReceiveBeginPlay`
  (bind _returnvalue (`GameplayStatics.GetActorOfClass` "/Game/FirstPerson/Blueprints/BP_FirstPersonCharacter.BP_FirstPersonCharacter_C"))
  (set `self.PlayerRef` _returnvalue)
  (`MeshComponent.SetScalarParameterValueOnMaterials` (`self.SM_Beacon_01_NeonBot3`) "Brightness" 3.0)
  (`MeshComponent.SetScalarParameterValueOnMaterials` (`self.SM_Beacon_01_NeonTop3`) "Brightness" 3.0)
  (`MeshComponent.SetScalarParameterValueOnMaterials` (`self.SM_Beacon_01_NeonBot2`) "Brightness" 3.0)
  (`MeshComponent.SetScalarParameterValueOnMaterials` (`self.SM_Beacon_01_NeonTop2`) "Brightness" 3.0)
  (`MeshComponent.SetScalarParameterValueOnMaterials` (`self.SM_Beacon_01_NeonBot1`) "Brightness" 3.0)
  (`MeshComponent.SetScalarParameterValueOnMaterials` (`self.SM_Beacon_01_NeonTop1`) "Brightness" 3.0)
  (set `self.DefaultPos` (`SceneComponent.K2_GetComponentLocation` (`self.DefaultSceneRoot`)))
  (`SkeletalMeshComponent.PlayAnimation` (`self.Beacon`) "/Game/Anim/Anim_Pyramid_idle.Anim_Pyramid_idle" true))

(event `Open`
  ;[0.1503 1 0 1 32] OPEN ANIMATION
  (if (not (`self.Open?`))
    (set `self.Open?` true)
    (`ActorComponent.Activate` (`self.NS_Beacon_Ceinture`) true)
    (`SkeletalMeshComponent.PlayAnimation` (`self.Beacon`) "/Game/VFX/Meshs/Anim_Pyramid_Action_Anim.Anim_Pyramid_Action_Anim" false)
    (`KismetSystemLibrary.Delay` 2.0)
    (`ActorComponent.Deactivate` (`self.NS_Beacon_Ceinture`))
    (`KismetSystemLibrary.Delay` 1.5)
    (`self.Desactivation`)))

(event `Activation`
  ;[1 0.6133 0 1 32] ACTIVATION
  (`/Engine/EditorBlueprintResources/StandardMacros.DoOnce` false
    (:`Completed`
      (`self.Open`))))

(event `Desactivation`
  ;[1 0 0.03936 1 32] DESACTIVATION
  (`MeshComponent.SetScalarParameterValueOnMaterials` (`self.SM_Beacon_01_NeonBot1`) "Brightness" 0.5)
  (`MeshComponent.SetScalarParameterValueOnMaterials` (`self.SM_Beacon_01_NeonTop1`) "Brightness" 0.5)
  (`KismetSystemLibrary.Delay` 0.2)
  (`MeshComponent.SetScalarParameterValueOnMaterials` (`self.SM_Beacon_01_NeonBot2`) "Brightness" 0.5)
  (`MeshComponent.SetScalarParameterValueOnMaterials` (`self.SM_Beacon_01_NeonTop2`) "Brightness" 0.5)
  (`KismetSystemLibrary.Delay` 0.2)
  (`MeshComponent.SetScalarParameterValueOnMaterials` (`self.SM_Beacon_01_NeonBot3`) "Brightness" 0.5)
  (`MeshComponent.SetScalarParameterValueOnMaterials` (`self.SM_Beacon_01_NeonTop3`) "Brightness" 0.5)
  ;[1 1 1] Fly Away
  (`KismetSystemLibrary.Delay` 0.5)
  (`MeshComponent.SetScalarParameterValueOnMaterials` (`self.SM_Beacon_01_NeonBot1`) "Brightness" 3.0)
  (`MeshComponent.SetScalarParameterValueOnMaterials` (`self.SM_Beacon_01_NeonTop1`) "Brightness" 3.0)
  (`MeshComponent.SetScalarParameterValueOnMaterials` (`self.SM_Beacon_01_NeonBot2`) "Brightness" 3.0)
  (`MeshComponent.SetScalarParameterValueOnMaterials` (`self.SM_Beacon_01_NeonTop2`) "Brightness" 3.0)
  (`MeshComponent.SetScalarParameterValueOnMaterials` (`self.SM_Beacon_01_NeonBot3`) "Brightness" 3.0)
  (`MeshComponent.SetScalarParameterValueOnMaterials` (`self.SM_Beacon_01_NeonTop3`) "Brightness" 3.0)
  (`SceneComponent.SetVisibility` (`self.SM_Beacon_01_NeonBot2`) false false)
  (`SceneComponent.SetVisibility` (`self.SM_Beacon_01_NeonTop2`) false false)
  (`SceneComponent.SetVisibility` (`self.SM_Beacon_01_NeonBot1`) false false)
  (`SceneComponent.SetVisibility` (`self.SM_Beacon_01_NeonTop1`) false false)
  (`SceneComponent.SetVisibility` (`self.SM_Beacon_01_NeonBot3`) false false)
  (`SceneComponent.SetVisibility` (`self.SM_Beacon_01_NeonTop3`) false false)
  (`SceneComponent.SetVisibility` (`self.SM_Beacon_01_Center`) false false)
  (`SkeletalMeshComponent.PlayAnimation` (`self.Beacon`) "/Game/Anim/Anim_Pyramid_Envole.Anim_Pyramid_Envole" false)
  (`KismetSystemLibrary.Delay` 3.5)
  (`self.K2_DestroyActor`))

(event `self.Sphere.OnComponentBeginOverlap`
  (params (OverlappedComponent :type "PrimitiveComponent Object Reference") (OtherActor :type "Actor Object Reference") (OtherComp :type "PrimitiveComponent Object Reference") (OtherBodyIndex :type Integer) (bFromSweep :type Boolean) (SweepResult :type "HitResult Structure (by ref)"))
  ;[1 1 1] Hitbox Interaction
  (cast `/Game/FirstPerson/Blueprints/BP_FirstPersonCharacter` OtherActor)
  (`self.Charge`)
  (`self.AppearZoneMat`))

(event `AppearZoneMat`
  (bind (_direction _newtrack_0) (`Timeline|MaterialTL` :!label _label)
    (:`Update`
      (`MaterialInstanceDynamic.SetScalarParameterValue` (`self.ZoneMaterial`) "Alpha" (`KismetMathLibrary.Lerp` 0.0 1.0 _newtrack_0)))))

(event `DisappearZoneMat`
  (goto _label :!via `Reverse`))

(event `self.Sphere.OnComponentEndOverlap`
  (params (OverlappedComponent :type "PrimitiveComponent Object Reference") (OtherActor :type "Actor Object Reference") (OtherComp :type "PrimitiveComponent Object Reference") (OtherBodyIndex :type Integer))
  ;[1 1 1] Hitbox Interaction
  (cast `/Game/FirstPerson/Blueprints/BP_FirstPersonCharacter` OtherActor)
  (`self.Discharge`)
  (`self.DisappearZoneMat`))

(event `Charge`
  (bind _mat_neontop1 (`self.Mat_NeonTop1`))
  (bind _mat_neonbot2 (`self.Mat_NeonBot2`))
  ;[1 1 1] Charge Handle
  (if (not (`self.Charged`))
    (`TimelineComponent.SetPlayRate` (`self.Timeline`) 3.0)
    (bind (_direction _newtrack_0) (`Timeline|Timeline` :!label _label_2)
      (:`Update`
        (set `self.ChargePercent` (`KismetMathLibrary.Lerp` 0.0 100.0 _newtrack_0))
        (if (>= _newtrack_0 0.3)
          (`MaterialInstanceDynamic.SetVectorParameterValue` (`self.Mat_NeonTop3`) "BaseColor" (struct :`G` 0.808633 :`B` 1.0 :`A` 1.0))
          (`MaterialInstanceDynamic.SetVectorParameterValue` (`self.Mat_NeonBot3`) "BaseColor" (struct :`G` 0.808633 :`B` 1.0 :`A` 1.0))
          (else
            (`MaterialInstanceDynamic.SetVectorParameterValue` (`self.Mat_NeonBot3`) "BaseColor" (struct :`R` 1.0 :`G` 0.01845 :`A` 1.0))
            (`MaterialInstanceDynamic.SetVectorParameterValue` (`self.Mat_NeonTop3`) "BaseColor" (struct :`R` 1.0 :`G` 0.01845 :`A` 1.0))))
        (if (>= _newtrack_0 0.6)
          (`MaterialInstanceDynamic.SetVectorParameterValue` _mat_neonbot2 "BaseColor" (struct :`G` 0.808633 :`B` 1.0 :`A` 1.0))
          (`MaterialInstanceDynamic.SetVectorParameterValue` (`self.Mat_NeonTop2`) "BaseColor" (struct :`G` 0.808633 :`B` 1.0 :`A` 1.0))
          (else
            (`MaterialInstanceDynamic.SetVectorParameterValue` _mat_neonbot2 "BaseColor" (struct :`R` 1.0 :`G` 0.01845 :`A` 1.0))
            (`MaterialInstanceDynamic.SetVectorParameterValue` (`self.Mat_NeonTop2`) "BaseColor" (struct :`R` 1.0 :`G` 0.01845 :`A` 1.0))))
        (if (>= _newtrack_0 0.99)
          (`MaterialInstanceDynamic.SetVectorParameterValue` _mat_neontop1 "BaseColor" (struct :`G` 0.808633 :`B` 1.0 :`A` 1.0))
          (`MaterialInstanceDynamic.SetVectorParameterValue` (`self.Mat_NeonBot1`) "BaseColor" (struct :`G` 0.808633 :`B` 1.0 :`A` 1.0))
          (`MaterialInstanceDynamic.SetVectorParameterValue` (`self.Mat_BeaconCenter1`) "BaseColor" (struct :`G` 0.808633 :`B` 1.0 :`A` 1.0))
          (else
            (`MaterialInstanceDynamic.SetVectorParameterValue` _mat_neontop1 "BaseColor" (struct :`R` 1.0 :`G` 0.01845 :`A` 1.0))
            (`MaterialInstanceDynamic.SetVectorParameterValue` (`self.Mat_NeonBot1`) "BaseColor" (struct :`R` 1.0 :`G` 0.01845 :`A` 1.0))
            (`MaterialInstanceDynamic.SetVectorParameterValue` (`self.Mat_BeaconCenter1`) "BaseColor" (struct :`R` 1.0 :`G` 0.01845 :`A` 1.0)))))
      (:`Finished`
        (if (>= (`self.ChargePercent`) 100.0)
          (set `self.Charged` true)
          (`self.DisappearZoneMat`)
          (`KismetSystemLibrary.Delay` 1.0)
          (`/Game/FirstPerson/Blueprints/BP_FirstPersonCharacter.CheckVictory` (`self.PlayerRef`) self)
          (`self.Activation`))))))

(event `Discharge`
  ;[1 1 1] Charge Handle
  (if (not (`self.Charged`))
    (`TimelineComponent.SetPlayRate` (`self.Timeline`) 1.0)
    (goto _label_2 :!via `Reverse`)))

(fn `UserConstructionScript`
  (bind _returnvalue (`PrimitiveComponent.CreateDynamicMaterialInstance` (`self.Sphere1`) 0 null "None"))
  (bind _output_get (set `self.ZoneMaterial` _returnvalue))
  (`MaterialInstanceDynamic.SetScalarParameterValue` _output_get "Alpha" 0.0)
  (bind _returnvalue_2 (`PrimitiveComponent.CreateDynamicMaterialInstance` (`self.SM_Beacon_01_NeonBot2`) 0 null "None"))
  (set `self.Mat_NeonBot2` _returnvalue_2)
  (bind _returnvalue_3 (`PrimitiveComponent.CreateDynamicMaterialInstance` (`self.SM_Beacon_01_NeonBot1`) 0 null "None"))
  (set `self.Mat_NeonBot1` _returnvalue_3)
  (bind _returnvalue_4 (`PrimitiveComponent.CreateDynamicMaterialInstance` (`self.SM_Beacon_01_NeonBot3`) 0 null "None"))
  (set `self.Mat_NeonBot3` _returnvalue_4)
  (bind _returnvalue_5 (`PrimitiveComponent.CreateDynamicMaterialInstance` (`self.SM_Beacon_01_NeonTop3`) 0 null "None"))
  (set `self.Mat_NeonTop3` _returnvalue_5)
  (bind _returnvalue_6 (`PrimitiveComponent.CreateDynamicMaterialInstance` (`self.SM_Beacon_01_Center`) 0 null "None"))
  (set `self.Mat_BeaconCenter1` _returnvalue_6)
  (bind _returnvalue_7 (`PrimitiveComponent.CreateDynamicMaterialInstance` (`self.SM_Beacon_01_NeonTop2`) 0 null "None"))
  (set `self.Mat_NeonTop2` _returnvalue_7)
  (bind _returnvalue_8 (`PrimitiveComponent.CreateDynamicMaterialInstance` (`self.SM_Beacon_01_NeonTop1`) 0 null "None"))
  (set `self.Mat_NeonTop1` _returnvalue_8)
  (`MaterialInstanceDynamic.SetVectorParameterValue` (`self.Mat_NeonBot3`) "BaseColor" (struct :`R` 1.0 :`G` 0.01845 :`A` 1.0))
  (`MaterialInstanceDynamic.SetVectorParameterValue` (`self.Mat_NeonBot2`) "BaseColor" (struct :`R` 1.0 :`G` 0.01845 :`A` 1.0))
  (`MaterialInstanceDynamic.SetVectorParameterValue` (`self.Mat_NeonBot1`) "BaseColor" (struct :`R` 1.0 :`G` 0.01845 :`A` 1.0))
  (`MaterialInstanceDynamic.SetVectorParameterValue` (`self.Mat_BeaconCenter1`) "BaseColor" (struct :`R` 1.0 :`G` 0.01845 :`A` 1.0))
  (`MaterialInstanceDynamic.SetVectorParameterValue` (`self.Mat_NeonTop3`) "BaseColor" (struct :`R` 1.0 :`G` 0.01845 :`A` 1.0))
  (`MaterialInstanceDynamic.SetVectorParameterValue` (`self.Mat_NeonTop2`) "BaseColor" (struct :`R` 1.0 :`G` 0.01845 :`A` 1.0))
  (`MaterialInstanceDynamic.SetVectorParameterValue` (`self.Mat_NeonTop1`) "BaseColor" (struct :`R` 1.0 :`G` 0.01845 :`A` 1.0)))