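; BP_SandWave is a VFX actor that sends a Niagara-style sand current effect repeatedly along a referenced spline.
; On BeginPlay it activates the effect and starts a timeline at a start offset, with a play rate randomized once from Duration.
; Each update moves the actor to the spline position at the timeline's value.
; On finish, it deactivates the effect, waits a randomized delay, then replays from the start.
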(event `self.ReceiveBeginPlay`
  (`self.ActivateWave`))

(event `ActivateWave`
  (bind _timeline_displacement (`self.Timeline_Displacement`))
  ;[0.3461 1 0 1 32] ACTIVATION
  (`ActorComponent.Activate` (`self.NS CourantSand`) false)
  (`TimelineComponent.SetPlayRate` _timeline_displacement (/ 1.0 (* (`self.Duration`) (`KismetMathLibrary.RandomFloat`))))
  (`TimelineComponent.SetNewTime` _timeline_displacement (`self.NSStartOffset`))
  (bind (_direction _alongaxis) (`Timeline|Timeline_Displacement` :!label _label)
    (:`Update`
      (`self.K2_SetActorLocation` (`SplineComponent.GetLocationAtTime` (`/Game/VFX/Blueprints/BP_SplineSand.SplinePass` (`self.SplineSandRef`)) _alongaxis "World" false)))
    (:`Finished`
      (`ActorComponent.Deactivate` (`self.NS CourantSand`))
      (`KismetSystemLibrary.Delay` (+ (* (`KismetMathLibrary.RandomFloat`) (`self.Delay`)) 1.0))
      (`ActorComponent.Activate` (`self.NS CourantSand`) false)
      (goto _label :!via `PlayFromStart`))))

(fn `UserConstructionScript`)