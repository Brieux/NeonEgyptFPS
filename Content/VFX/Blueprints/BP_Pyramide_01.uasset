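; Pyramid VFX actor that opens once when the jump input (IA_Jump) triggers, then spins its central sphere.
; A DoOnce-guarded timeline pushes the four outer pyramid parts outward and down while setting their pitch, and raises the sphere.
; Timeline offsets are added to current world transforms on every update, so movement accumulates.
; When the timeline finishes, Opened is set and Tick yaws the sphere by a fixed step each frame.
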(event `EnhancedInput|/Game/FirstPerson/Input/Actions/IA_Jump`
  (params (ActionValue :type Boolean) (ElapsedSeconds :type "Float (double-precision)") (TriggeredSeconds :type "Float (double-precision)") (InputAction :type "InputAction Object Reference" :default "/Game/FirstPerson/Input/Actions/IA_Jump.IA_Jump"))
  (:`Triggered`
    (`self.OpenPE`)))

(event `self.ReceiveTick`
  (params (DeltaSeconds :type "Float (single-precision)"))
  (`self.RotatePE`))

(event `RotatePE`
  (bind (_returnvalue_roll _returnvalue_pitch _returnvalue_yaw) (`KismetMathLibrary.BreakRotator` (`SceneComponent.K2_GetComponentRotation` (`self.Sphere`))))
  ;[0.1455 1 0 1 32] ANIM ROTATION
  (if (`self.Opened`)
    (`SceneComponent.K2_SetWorldRotation` (`self.Sphere`) (`KismetMathLibrary.MakeRotator` 0.0 0.0 (+ _returnvalue_yaw 1.0)) false false)))

(event `OpenPE`
  (bind _pyramide2_parte1_ext2 (`self.Pyramide2_Parte1_Ext2`))
  (bind _pyramide2_parte1_ext3 (`self.Pyramide2_Parte1_Ext3`))
  (bind _sphere (`self.Sphere`))
  (bind _pyramide2_parte1_ext4 (`self.Pyramide2_Parte1_Ext4`))
  (bind _pyramide2_parte1_ext1 (`self.Pyramide2_Parte1_Ext1`))
  (bind _returnvalue (`SceneComponent.K2_GetComponentToWorld` _pyramide2_parte1_ext4))
  (bind _returnvalue_2 (`SceneComponent.K2_GetComponentToWorld` _pyramide2_parte1_ext1))
  (bind _returnvalue_3 (`SceneComponent.K2_GetComponentToWorld` _pyramide2_parte1_ext2))
  (bind _returnvalue_4 (`SceneComponent.K2_GetComponentToWorld` _pyramide2_parte1_ext3))
  (bind (_returnvalue_x _returnvalue_y _returnvalue_z) (`KismetMathLibrary.BreakVector` (`SceneComponent.K2_GetComponentLocation` _sphere)))
  ;[1 0.9244 0 1 32] ANIM OPENNING ACTIVATION
  (`/Engine/EditorBlueprintResources/StandardMacros.DoOnce` false
    (:`Completed`
      (bind (_direction _pitchvalue _displacementhorizontale _displacementverticale) (`Timeline|Timeline_OpenPE` :!via `PlayFromStart`)
        (:`Update`
          (`SceneComponent.K2_SetWorldTransform` _pyramide2_parte1_ext1 (`KismetMathLibrary.MakeTransform` (`KismetMathLibrary.MakeVector` (.x (.location _returnvalue_2)) (- (.y (.location _returnvalue_2)) _displacementhorizontale) (- (.z (.location _returnvalue_2)) _displacementverticale)) (`KismetMathLibrary.MakeRotator` (.roll (.rotation _returnvalue_2)) _pitchvalue (.yaw (.rotation _returnvalue_2))) (10.0 10.0 10.0)) false false)
          (`SceneComponent.K2_SetWorldTransform` _pyramide2_parte1_ext2 (`KismetMathLibrary.MakeTransform` (`KismetMathLibrary.MakeVector` (- (.x (.location _returnvalue_3)) _displacementhorizontale) (.y (.location _returnvalue_3)) (- (.z (.location _returnvalue_3)) _displacementverticale)) (`KismetMathLibrary.MakeRotator` (.roll (.rotation _returnvalue_3)) _pitchvalue (.yaw (.rotation _returnvalue_3))) (10.0 10.0 10.0)) false false)
          (`SceneComponent.K2_SetWorldTransform` _pyramide2_parte1_ext3 (`KismetMathLibrary.MakeTransform` (`KismetMathLibrary.MakeVector` (.x (.location _returnvalue_4)) (+ (.y (.location _returnvalue_4)) _displacementhorizontale) (- (.z (.location _returnvalue_4)) _displacementverticale)) (`KismetMathLibrary.MakeRotator` (.roll (.rotation _returnvalue_4)) _pitchvalue (.yaw (.rotation _returnvalue_4))) (10.0 10.0 10.0)) false false)
          (`SceneComponent.K2_SetWorldTransform` _pyramide2_parte1_ext4 (`KismetMathLibrary.MakeTransform` (`KismetMathLibrary.MakeVector` (+ (.x (.location _returnvalue)) _displacementhorizontale) (.y (.location _returnvalue)) (- (.z (.location _returnvalue)) _displacementverticale)) (`KismetMathLibrary.MakeRotator` (.roll (.rotation _returnvalue)) _pitchvalue (.yaw (.rotation _returnvalue))) (10.0 10.0 10.0)) false false)
          (`SceneComponent.K2_SetWorldLocation` _sphere (`KismetMathLibrary.MakeVector` _returnvalue_x _returnvalue_y (+ _returnvalue_z _displacementverticale)) false false))
        (:`Finished`
          (set `self.Opened` true))))))

(fn `UserConstructionScript`)