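; BP_Pyramide is a pyramid actor animated vertically with timelines.
; The construction script stores the root's position, and from BeginPlay a looping Ascension timeline offsets the root's height from that base by a lerp.
; A separate Chute event, not called in this graph, lowers the upper part (PyramideHaut) cumulatively on each timeline update, then restarts Ascension.
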(event `Ascension`
  (bind (_posebase_x _posebase_y _posebase_z) (`KismetMathLibrary.BreakVector` (`self.PoseBase`)))
  (bind (_direction _displacementverticale) (`Timeline|Timeline_0` :!via `PlayFromStart`)
    (:`Update`
      (`SceneComponent.K2_SetWorldLocation` (`self.DefaultSceneRoot`) (`KismetMathLibrary.MakeVector` _posebase_x _posebase_y (+ _posebase_z (`KismetMathLibrary.Lerp` 0.0 200.0 _displacementverticale))) false false))
    (:`Finished`
      (`self.Ascension`))))

(event `self.ReceiveBeginPlay`
  (`self.Ascension`))

(event `Chute`
  (bind _pyramide_haut (`self.Pyramide_Haut`))
  (bind (_returnvalue_x _returnvalue_y _returnvalue_z) (`KismetMathLibrary.BreakVector` (`SceneComponent.K2_GetComponentLocation` _pyramide_haut)))
  (bind (_direction _displacementverticale) (`Timeline|Timeline_1` :!via `PlayFromStart`)
    (:`Update`
      (`SceneComponent.K2_SetWorldLocation` _pyramide_haut (`KismetMathLibrary.MakeVector` _returnvalue_x _returnvalue_y (- _returnvalue_z (* _displacementverticale 1.0))) false false))
    (:`Finished`
      (`self.Ascension`))))

(fn `UserConstructionScript`
  (set `self.PoseBase` (`SceneComponent.K2_GetComponentLocation` (`self.DefaultSceneRoot`))))