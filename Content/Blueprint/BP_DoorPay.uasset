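; BP_DoorPay is a purchasable door that the player opens by spending score points, activating its assigned spawners.
; Interact checks PlayerScore against DoorPrice, then deducts it, plays a sound, and hides and disables collision on itself and ConnectedDoors, or prints a message if funds are short.
; The construction script writes the price onto two text labels, which show only while the player overlaps PriceShowTrigger.
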(event `self.ReceiveBeginPlay`
  (bind _asbp_first_person_character (cast `/Game/FirstPerson/Blueprints/BP_FirstPersonCharacter` (`GameplayStatics.GetPlayerPawn` 0)))
  (set `self.PlayerRef` _asbp_first_person_character))

(event `/Game/Blueprint/BPI_Interact.Interact`
  (bind _connecteddoors (`self.ConnectedDoors`))
  (bind _playerref (`self.PlayerRef`))
  (bind _enough_ (`self.CheckBalance` (`/Game/FirstPerson/Blueprints/BP_FirstPersonCharacter.PlayerScore` _playerref)))
  (if _enough_
    (`self.Pay` _playerref)
    (`GameplayStatics.PlaySoundAtLocation` "/Game/Audio/AMB/AMB_PayDoor.AMB_PayDoor" (`SceneComponent.K2_GetComponentLocation` (`self.DefaultSceneRoot`)) (struct) 1.0 1.0 0.0 null null null null)
    (`self.SetActorEnableCollision` _connecteddoors false)
    (`self.SetActorHiddenInGame` _connecteddoors true)
    (`self.SetActorEnableCollision` false)
    (`self.SetActorHiddenInGame` true)
    (for _array_element (`self.SpawnerToActivate`)
      (`/Game/Blueprint/BP_SpawnerAScaraB.ActivateSpawner` _array_element))
    (else
      (`KismetSystemLibrary.PrintString` "(Door) Not enough money."))))

(event `self.PriceShowTrigger.OnComponentBeginOverlap`
  (params (OverlappedComponent :type "PrimitiveComponent Object Reference") (OtherActor :type "Actor Object Reference") (OtherComp :type "PrimitiveComponent Object Reference") (OtherBodyIndex :type Integer) (bFromSweep :type Boolean) (SweepResult :type "HitResult Structure (by ref)"))
  (cast `/Game/FirstPerson/Blueprints/BP_FirstPersonCharacter` OtherActor)
  (`SceneComponent.SetHiddenInGame` (`self.DoorPrice1`) false false)
  (`SceneComponent.SetHiddenInGame` (`self.DoorPrice0`) false false))

(event `self.PriceShowTrigger.OnComponentEndOverlap`
  (params (OverlappedComponent :type "PrimitiveComponent Object Reference") (OtherActor :type "Actor Object Reference") (OtherComp :type "PrimitiveComponent Object Reference") (OtherBodyIndex :type Integer))
  (cast `/Game/FirstPerson/Blueprints/BP_FirstPersonCharacter` OtherActor)
  (`SceneComponent.SetHiddenInGame` (`self.DoorPrice0`) true false)
  (`SceneComponent.SetHiddenInGame` (`self.DoorPrice1`) true false))

(fn `CheckBalance`
  (params (Balance :type Integer))
  (returns (`Enough?` :type Boolean))
  (return (>= Balance (`self.DoorPrice`))))

(fn `Pay`
  (params (Player :type "/Game/FirstPerson/Blueprints/BP_FirstPersonCharacter Object Reference"))
  (set `/Game/FirstPerson/Blueprints/BP_FirstPersonCharacter.PlayerScore` (- (`/Game/FirstPerson/Blueprints/BP_FirstPersonCharacter.PlayerScore` Player) (`self.DoorPrice`)) Player))

(fn `UserConstructionScript`
  (`TextRenderComponent.K2_SetText` (`self.DoorPrice1`) (`|FormatText` "Spend {price}p to open" (`KismetTextLibrary.Conv_IntToText` (`self.DoorPrice`) false false)))
  (`TextRenderComponent.K2_SetText` (`self.DoorPrice0`) (`|FormatText` "Spend {price}p to open" (`KismetTextLibrary.Conv_IntToText` (`self.DoorPrice`) false false))))