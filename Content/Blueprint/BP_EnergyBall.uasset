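; Energy pickup ball that flies to the first-person character and refills the energy on its ABMarkInChain.
; SphereActivate starts a timeline that lerps the ball from its spawn location to the player's live position, then destroys it.
; Alongside it, a looping timer at frame-delta interval moves energy from EnergyStored into the player's clamped EnergyAvailable at SpeedToRefill.
; The depleted-or-full check has no effect, so refilling continues until destruction.
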(event `self.ReceiveBeginPlay`
  (set `self.DefaultPose` (`self.K2_GetActorLocation`))
  (`SceneComponent.SetWorldScale3D` (`self.Sphere`) (0.4 0.4 0.4)))

(event `SphereActivate`
  (params (`As BP First Person Character` :type "/Game/FirstPerson/Blueprints/BP_FirstPersonCharacter Object Reference"))
  (set `self.As BP First Person Character` `As BP First Person Character`)
  (`KismetSystemLibrary.K2_SetTimerDelegate` (delegate `refillEnergy`) (`GameplayStatics.GetWorldDeltaSeconds`) true)
  (bind (_direction _newtrack_0) (`Timeline|GoToPlayer` :!via `PlayFromStart`)
    (:`Update`
      (`self.K2_SetActorLocation` (`KismetMathLibrary.VLerp` (`self.DefaultPose`) (`self.K2_GetActorLocation` (`self.As BP First Person Character`)) _newtrack_0)))
    (:`Finished`
      (`self.K2_DestroyActor`))))

(event `refillEnergy`
  (bind _returnvalue (* (`GameplayStatics.GetWorldDeltaSeconds`) (`self.SpeedToRefill`)))
  (bind _ab_markinchain (`/Game/FirstPerson/Blueprints/BP_FirstPersonCharacter.AB_MarkInChain` (`self.As BP First Person Character`)))
  (bind _output_get (set `/Game/FirstPerson/Blueprints/Abilities/AB_MarkInChain.EnergyAvailable` (`KismetMathLibrary.FClamp` (+ (`/Game/FirstPerson/Blueprints/Abilities/AB_MarkInChain.EnergyAvailable` _ab_markinchain) _returnvalue) 0.0 100.0) _ab_markinchain))
  (bind _output_get_2 (set `self.EnergyStored` (- (`self.EnergyStored`) _returnvalue)))
  (if (or (<= _output_get_2 0.0) (>= _output_get 100.0))
    _))

(fn `UserConstructionScript`)