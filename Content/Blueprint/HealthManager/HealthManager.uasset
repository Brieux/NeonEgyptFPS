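; HealthManager is a component that tracks its owning entity's health and death state.
; A single ManageHealth event switches on an action to remove, add, set or restore health, or change the maximum, keeping full health full.
; Remove and Set update IsDead, and zero health calls EventDeath, which sends DieMessage to the owner with the InChain flag.
; Only Remove and Add clamp the value, and debug text reports health and death.
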(event `ManageHealth`
  (params (Action :type "/Game/Blueprint/HealthManager/E_HealthAction Enum" :default "NewEnumerator1") (Value :type "Float (double-precision)") (`In Chain?` :type Boolean))
  (bind _health (`self.Health`))
  (bind _maximumhealth (`self.MaximumHealth`))
  (bind _returnvalue (- _health Value))
  (bind _returnvalue_2 (+ _health Value))
  (set `self.In Chain?` `In Chain?`)
  (switch `/Game/Blueprint/HealthManager/E_HealthAction` Action
    (:`NewEnumerator1`
      (set `self.Health` (`KismetMathLibrary.SelectFloat` 0.0 _returnvalue (< _returnvalue 0.0)))
      (if (== (`self.Health`) 0.0) :!label _label
        (set `self.isDead` true)
        (`self.EventDeath`)
        (else
          (set `self.isDead` false)))
      (`KismetSystemLibrary.PrintText` (`|FormatText` "(HealthManager) CurrentHealth : {hp}/{mhp}" (`self.Health`) (`self.MaximumHealth`)) :!label _label_2))
    (:`NewEnumerator0`
      (set `self.Health` (`KismetMathLibrary.SelectFloat` _maximumhealth _returnvalue_2 (> _returnvalue_2 _maximumhealth)))
      (goto _label_2))
    (:`NewEnumerator2`
      (set `self.Health` Value)
      (goto _label))
    (:`NewEnumerator3`
      (set `self.Health` (`self.MaximumHealth`))
      (goto _label_2))
    (:`NewEnumerator4`
      (if (== (`self.Health`) (`self.MaximumHealth`))
        (bind _output_get (set `self.MaximumHealth` Value))
        (`self.ManageHealth` "NewEnumerator2" _output_get)
        (else
          (set `self.MaximumHealth` Value))))))

(fn `EventDeath`
  (`KismetSystemLibrary.PrintText` (`|FormatText` "(HealthManager) Entity {e} is dead." (`KismetSystemLibrary.GetObjectName` (`self.GetOwner`))))
  (message `/Game/Blueprint/HealthManager/BPI_HealthInteraction.Die` (`self.GetOwner`) (`self.In Chain?`)))