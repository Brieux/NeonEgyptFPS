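; Purchasable altar (Autel) whose AutelType sets its mesh and price, selling blessings for player score via Interact.
; TryBuyAutel charges the player and records the Benediction; every type except Anubis is one-time.
; Anubis gambles on shifting odds to raise or reset energy regen, Horus calls the player's health handler, and Teleport moves the player away for 15 seconds.
; Khnum and Thoth have prices but no effect.
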(event `self.ReceiveBeginPlay`
  (bind _staticmesh (`self.StaticMesh`))
  (bind _asbp_first_person_character (cast `/Game/FirstPerson/Blueprints/BP_FirstPersonCharacter` (`GameplayStatics.GetPlayerCharacter` 0)))
  (set `self.As BP First Person Character` _asbp_first_person_character)
  (set `self.Price` (select `/Game/Blueprint/E_AutelType` (`self.AutelType`) :`NewEnumerator0` 1800 :`NewEnumerator1` 2500 :`NewEnumerator2` 3000 :`NewEnumerator4` 25000))
  (switch `/Game/Blueprint/E_AutelType` (`self.AutelType`)
    (:`NewEnumerator0`
      (`StaticMeshComponent.SetStaticMesh` _staticmesh "/Game/Assets_3D/Statues/Anubis/Anubis_low.Anubis_low"))
    (:`NewEnumerator1`
      (`StaticMeshComponent.SetStaticMesh` _staticmesh "/Game/Assets_3D/Statues/Horus/Horus_low.Horus_low"))
    (:`NewEnumerator4`
      (`SceneComponent.SetHiddenInGame` _staticmesh true false))))

(event `/Game/Blueprint/BPI_Interact.Interact`
  (`self.Try Buy Autel`))

(event `GoBack`
  (`KismetSystemLibrary.Delay` 15.0)
  (`self.K2_SetActorLocation` (`self.As BP First Person Character`) (351.0 324.0 268.0) false true))

(fn `AnubisEffect`
  (returns (Success :type Boolean) (CurrentStack :type Integer))
  (bind _as_bp_first_person_character (`self.As BP First Person Character`))
  (bind _counterbeneanubis (`/Game/FirstPerson/Blueprints/BP_FirstPersonCharacter.CounterBeneAnubis` _as_bp_first_person_character))
  (bind _counterbeneanubis_2 (`/Game/FirstPerson/Blueprints/BP_FirstPersonCharacter.CounterBeneAnubis` _as_bp_first_person_character))
  (if (> _counterbeneanubis 1)
    (set `/Game/FirstPerson/Blueprints/BP_FirstPersonCharacter.CounterBeneAnubis` (- _counterbeneanubis 1) _as_bp_first_person_character))
  (if (<= (`KismetMathLibrary.RandomIntegerInRange` 1 10) _counterbeneanubis)
    ;[1 1 1] Positif
    (set `/Game/FirstPerson/Blueprints/BP_FirstPersonCharacter.EnergyRegenRate` (+ (`/Game/FirstPerson/Blueprints/BP_FirstPersonCharacter.EnergyRegenRate` _as_bp_first_person_character) 0.1) _as_bp_first_person_character)
    (return true _counterbeneanubis_2)
    (else
      ;[1 1 1] Négatif
      (set `/Game/FirstPerson/Blueprints/BP_FirstPersonCharacter.EnergyRegenRate` 0.2 _as_bp_first_person_character)
      (set `/Game/FirstPerson/Blueprints/BP_FirstPersonCharacter.CounterBeneAnubis` (`KismetMathLibrary.Clamp` (+ _counterbeneanubis_2 4) 1 11) _as_bp_first_person_character)
      (return false _counterbeneanubis_2))))

(fn `Try Buy Autel`
  (returns (Succeed :type Boolean))
  (bind _auteltype (`self.AutelType`))
  (bind _as_bp_first_person_character (`self.As BP First Person Character`))
  (bind _as_bp_first_person_character_2 (`self.As BP First Person Character`))
  (bind _benediction_bene (break `/Game/Blueprint/Str_Benediction` (`/Game/FirstPerson/Blueprints/BP_FirstPersonCharacter.Benediction` (`self.As BP First Person Character`))))
  (bind _benediction_bene_2 (break `/Game/Blueprint/Str_Benediction` (`/Game/FirstPerson/Blueprints/BP_FirstPersonCharacter.Benediction` (`self.As BP First Person Character`))))
  (if (>= (`/Game/FirstPerson/Blueprints/BP_FirstPersonCharacter.PlayerScore` _as_bp_first_person_character_2) (`self.Price`))
    (if (`|EnumEquality` _auteltype "NewEnumerator0")
      _
      (elif (not (`BlueprintMapLibrary.Map_Find` _benediction_bene _auteltype))
        _
        (else
          (return false))))
    (`/Game/FirstPerson/Blueprints/BP_FirstPersonCharacter.ManagePoint` _as_bp_first_person_character_2 "NewEnumerator1" (`KismetMathLibrary.Conv_IntToDouble` (`self.Price`)))
    (`BlueprintMapLibrary.Map_Add` _benediction_bene_2 (`self.AutelType`) true)
    (switch `/Game/Blueprint/E_AutelType` (`self.AutelType`)
      (:`NewEnumerator0`
        (bind (_success _currentstack) (`self.AnubisEffect`))
        (`KismetSystemLibrary.PrintText` (`|FormatText` "(Anubis) Benediction result : Success is {s}, current chance with {r}0%, energyregen at {regen}/s" _success _currentstack (`/Game/FirstPerson/Blueprints/BP_FirstPersonCharacter.EnergyRegenRate` _as_bp_first_person_character)) true true (struct :`R` 1.0 :`G` 0.40335 :`A` 1.0) 4.0)
        (return true))
      (:`NewEnumerator1`
        (message `/Game/Blueprint/HealthManager/BPI_HealthInteraction.Manage Health` _as_bp_first_person_character "NewEnumerator4" 5.0 false)
        (return true))
      (:`NewEnumerator4`
        (`self.K2_SetActorLocation` (`self.As BP First Person Character`) (-25000.0 21800.0 -150.0) false true)
        (`self.GoBack`)))
    (else
      (return false))))

(fn `UserConstructionScript`
  (bind _auteltype (`self.AutelType`))
  (bind _staticmesh (`self.StaticMesh`))
  (set `self.Price` (select `/Game/Blueprint/E_AutelType` _auteltype :`NewEnumerator0` 1800 :`NewEnumerator1` 2500 :`NewEnumerator2` 3000))
  (switch `/Game/Blueprint/E_AutelType` _auteltype
    (:`NewEnumerator0`
      (`StaticMeshComponent.SetStaticMesh` _staticmesh "/Game/Assets_3D/Statues/Anubis/Anubis_low.Anubis_low"))
    (:`NewEnumerator1`
      (`StaticMeshComponent.SetStaticMesh` _staticmesh "/Game/Assets_3D/Statues/Horus/Horus_low.Horus_low"))))