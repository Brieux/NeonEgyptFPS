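; BP_Autel is an interactable altar that sells the player a god's blessing for score points.
; Its AutelType sets the price and, for Anubis and Horus, the mesh, both in construction and at BeginPlay.
; Interacting checks the player's score, charges it and records the blessing on the character.
; Anubis then sets a blessing counter and Horus sends a health message, while Khnum and Thoth have no extra effect.
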(event `self.ReceiveBeginPlay`
  (bind _staticmesh (`self.StaticMesh`))
  (bind _asbp_first_person_character (cast `/Game/FirstPerson/Blueprints/BP_FirstPersonCharacter` (`GameplayStatics.GetPlayerCharacter` 0)))
  (set `self.As BP First Person Character` _asbp_first_person_character)
  (set `self.Price` (select `/Game/Blueprint/E_AutelType` (`self.AutelType`) :`NewEnumerator0` 1800 :`NewEnumerator1` 2500 :`NewEnumerator2` 3000))
  (switch `/Game/Blueprint/E_AutelType` (`self.AutelType`)
    (:`NewEnumerator0`
      (`StaticMeshComponent.SetStaticMesh` _staticmesh "/Game/Assets_3D/Statues/Anubis/Anubis_low.Anubis_low"))
    (:`NewEnumerator1`
      (`StaticMeshComponent.SetStaticMesh` _staticmesh "/Game/Assets_3D/Statues/Horus/Horus_low.Horus_low"))))

(event `/Game/Blueprint/BPI_Interact.Interact`
  (`self.Try Buy Autel`))

(fn `Try Buy Autel`
  (returns (Succeed :type Boolean))
  (bind _as_bp_first_person_character (`self.As BP First Person Character`))
  (bind _as_bp_first_person_character_2 (`self.As BP First Person Character`))
  (bind _benediction_bene (break `/Game/Blueprint/Str_Benediction` (`/Game/FirstPerson/Blueprints/BP_FirstPersonCharacter.Benediction` _as_bp_first_person_character_2)))
  (if (>= (`/Game/FirstPerson/Blueprints/BP_FirstPersonCharacter.PlayerScore` _as_bp_first_person_character) (`self.Price`))
    (`/Game/FirstPerson/Blueprints/BP_FirstPersonCharacter.ManagePoint` _as_bp_first_person_character "NewEnumerator1" (`KismetMathLibrary.Conv_IntToDouble` (`self.Price`)))
    (`BlueprintMapLibrary.Map_Add` _benediction_bene (`self.AutelType`) true)
    (switch `/Game/Blueprint/E_AutelType` (`self.AutelType`)
      (:`NewEnumerator0`
        (set `/Game/FirstPerson/Blueprints/BP_FirstPersonCharacter.CounterBeneAnubis` 4 _as_bp_first_person_character_2))
      (:`NewEnumerator1`
        (message `/Game/Blueprint/HealthManager/BPI_HealthInteraction.Manage Health` (`self.As BP First Person Character`) "NewEnumerator4" 5.0 false)))
    (return true)
    (else
      (return false))))

(fn `UserConstructionScript`
  (bind _auteltype (`self.AutelType`))
  (bind _staticmesh (`self.StaticMesh`))
  (set `self.Price` (select `/Game/Blueprint/E_AutelType` _auteltype :`NewEnumerator0` 1800 :`NewEnumerator1` 2500 :`NewEnumerator2` 3000))
  (switch `/Game/Blueprint/E_AutelType` _auteltype
    (:`NewEnumerator0`
      (`StaticMeshComponent.SetStaticMesh` _staticmesh "/Game/Assets_3D/Statues/Anubis/Anubis_low.Anubis_low"))
    (:`NewEnumerator1`
      (`StaticMeshComponent.SetStaticMesh` _staticmesh "/Game/Assets_3D/Statues/Horus/Horus_low.Horus_low"))))