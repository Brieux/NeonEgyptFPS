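; Enemy character that runs BT_Enemy with the player as blackboard target and damages the player on box overlap.
; It can be marked into the player's numbered chain (ABMarkInChain), then trigger that chain's explosion and take chain-length-scaled reaction damage through HealthManager.
; Death awards points, with a growing bonus for chain kills, spawns Niagara effects and destroys the actor.
; Anubis sphere-trace mark propagation and widget billboarding exist but are disconnected.
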(event `self.ReceiveBeginPlay`
  (bind _returnvalue (`self.GetController`))
  (bind _returnvalue_2 (`GameplayStatics.GetPlayerCharacter` 0))
  (bind _asai_enemy (cast `/Game/Blueprint/IA_Component/AI_Enemy` _returnvalue))
  (`AIController.RunBehaviorTree` _asai_enemy "/Game/Blueprint/IA_Component/BT_Enemy.BT_Enemy")
  (`BlackboardComponent.SetValueAsObject` (`AIBlueprintHelperLibrary.GetBlackboard` _returnvalue) "PlayerRef" _returnvalue_2)
  (bind _asbp_first_person_character (cast `/Game/FirstPerson/Blueprints/BP_FirstPersonCharacter` _returnvalue_2))
  (set `self.As BP First Person Character` _asbp_first_person_character))

(event `self.ReceiveTick`
  (params (DeltaSeconds :type "Float (single-precision)")))

(event `/Game/Blueprint/BPI_Marquage.GetMarked`
  (params (IntegerInChain :type Integer))
  (set `self.IsInChainNumber` IntegerInChain)
  (`ActorComponent.Activate` (`self.NS_Selected1`) true)
  (`ActorComponent.Activate` (`self.NS_Selected`) true))

(event `/Game/Blueprint/BPI_Marquage.TriggerChain`
  (bind _output_get (set `self.Chain` (`/Game/FirstPerson/Blueprints/BP_FirstPersonCharacter.AB_MarkInChain` (`self.As BP First Person Character`))))
  (`/Game/FirstPerson/Blueprints/Abilities/AB_MarkInChain.ExploseChain` _output_get self)
  (`KismetSystemLibrary.DelayUntilNextTick`)
  (message `/Game/Blueprint/HealthManager/BPI_HealthInteraction.Die` self false))

(event `/Game/Blueprint/HealthManager/BPI_HealthInteraction.Die`
  (params (`inChain?` :type Boolean))
  (bind _as_bp_first_person_character (`self.As BP First Person Character`))
  (bind _chain (`self.Chain`))
  (set `self.Chain` (`/Game/FirstPerson/Blueprints/BP_FirstPersonCharacter.AB_MarkInChain` (`self.As BP First Person Character`)))
  (if `inChain?`
    (set `/Game/FirstPerson/Blueprints/Abilities/AB_MarkInChain.DieInChain` (+ (`/Game/FirstPerson/Blueprints/Abilities/AB_MarkInChain.DieInChain` _chain) 1) _chain)
    (`/Game/FirstPerson/Blueprints/BP_FirstPersonCharacter.ManagePoint` _as_bp_first_person_character "NewEnumerator0" (+ (`self.ValuePoint+`) (* (`/Game/FirstPerson/Blueprints/Abilities/AB_MarkInChain.DieInChain` (`self.Chain`)) 10.0)))
    (else
      (`/Game/FirstPerson/Blueprints/BP_FirstPersonCharacter.ManagePoint` _as_bp_first_person_character "NewEnumerator0" (`self.ValuePoint+`))))
  (`NiagaraFunctionLibrary.SpawnSystemAtLocation` "/Game/VFX/Niagara/NS_MobDeath.NS_MobDeath" (- (`SceneComponent.K2_GetComponentLocation` (`self.CapsuleComponent`)) (0.0 0.0 77.0)))
  (`self.DetachFromControllerPendingDestroy`)
  (`self.K2_DestroyActor`))

(event `/Game/Blueprint/HealthManager/BPI_HealthInteraction.Manage Health`
  (params (Action :type "/Game/Blueprint/HealthManager/E_HealthAction Enum" :default "NewEnumerator1") (Value :type "Float (double-precision)") (InChain :type Boolean))
  (`/Game/Blueprint/HealthManager/HealthManager.ManageHealth` (`self.HealthManager`) Action Value InChain))

(event `/Game/Blueprint/BPI_Marquage.ReactionChain`
  (params (NumberInChain :type Integer) (ChainLenght :type Integer))
  (`KismetSystemLibrary.PrintString` (`KismetSystemLibrary.GetDisplayName` self))
  (message `/Game/Blueprint/HealthManager/BPI_HealthInteraction.Manage Health` self "NewEnumerator1" (`KismetMathLibrary.Conv_IntToDouble` ChainLenght) true))

(event `self.Box.OnComponentBeginOverlap`
  (params (OverlappedComponent :type "PrimitiveComponent Object Reference") (OtherActor :type "Actor Object Reference") (OtherComp :type "PrimitiveComponent Object Reference") (OtherBodyIndex :type Integer) (bFromSweep :type Boolean) (SweepResult :type "HitResult Structure (by ref)"))
  (if (`KismetSystemLibrary.DoesImplementInterface` OtherActor "/Game/Blueprint/HealthManager/BPI_HealthInteraction.BPI_HealthInteraction_C")
    (bind _asbp_first_person_character (cast `/Game/FirstPerson/Blueprints/BP_FirstPersonCharacter` OtherActor))
    (message `/Game/Blueprint/HealthManager/BPI_HealthInteraction.Manage Health` _asbp_first_person_character "NewEnumerator1" 1.0 false)))

(fn `isAlreadyMarked?`
  (returns (Yes :type Boolean))
  (return (not (== (`self.IsInChainNumber`) -1))))

(fn `TryGetAnubisMarked`
  (bind _returnvalue (`self.K2_GetActorLocation`))
  (bind _as_bp_first_person_character (`self.As BP First Person Character`))
  (bind _as_bp_first_person_character_2 (`self.As BP First Person Character`))
  (bind _ab_markinchain (`/Game/FirstPerson/Blueprints/BP_FirstPersonCharacter.AB_MarkInChain` (`self.As BP First Person Character`)))
  (bind _returnvalue_2 (+ (`/Game/FirstPerson/Blueprints/Abilities/AB_MarkInChain.ValueInChain` _ab_markinchain) 1))
  (set `/Game/FirstPerson/Blueprints/BP_FirstPersonCharacter.CounterBeneAnubis` (- (`/Game/FirstPerson/Blueprints/BP_FirstPersonCharacter.CounterBeneAnubis` _as_bp_first_person_character) 1) _as_bp_first_person_character)
  (bind _outhits (`KismetSystemLibrary.SphereTraceMulti` :`Start` _returnvalue :`End` _returnvalue :`Radius` (`self.RadiusAnubisPropagate`) :`TraceChannel` "TraceTypeQuery3" :`DrawDebugType` "ForDuration"))
  (for _array_element _outhits
    (bind (_bblockinghit _binitialoverlap _time _distance _location _impactpoint _normal _impactnormal _physmat _hitactor) (`GameplayStatics.BreakHitResult` _array_element))
    (if (`KismetSystemLibrary.DoesImplementInterface` _hitactor "/Game/Blueprint/BPI_Marquage.BPI_Marquage_C")
      (bind _yes (message `/Game/Blueprint/BPI_Marquage.isAlreadyMarked?` _hitactor))
      (if (not _yes)
        (message `/Game/Blueprint/BPI_Marquage.GetMarked` _hitactor _returnvalue_2)
        (set `/Game/FirstPerson/Blueprints/Abilities/AB_MarkInChain.ValueInChain` _returnvalue_2 _ab_markinchain)
        (`KismetArrayLibrary.Array_AddUnique` (`/Game/FirstPerson/Blueprints/Abilities/AB_MarkInChain.Chain` _ab_markinchain) _hitactor)
        (set `/Game/FirstPerson/Blueprints/BP_FirstPersonCharacter.CounterBeneAnubis` (- (`/Game/FirstPerson/Blueprints/BP_FirstPersonCharacter.CounterBeneAnubis` _as_bp_first_person_character_2) 1) _as_bp_first_person_character_2)))))

(fn `UserConstructionScript`)